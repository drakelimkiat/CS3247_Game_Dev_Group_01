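; Frying pan that the player interacts with to place, take or swap unfinished BP_Food_Frying items on its snap point.
; Tick shows the level's first BP_FryingBar while food is on top, seeding progress from the food's remaining FoodProgress and starting sizzle audio.
; A looping Fry timer advances the bar and decrements FoodProgress until Tick calls FoodDone at full progress.
; Custom depth outlines the empty pan for valid food.
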(event `self.ReceiveBeginPlay`
  ;[1 1 1] On begin play set FryingBar.
  (bind _outactors (`GameplayStatics.GetAllActorsOfClass` "/Game/BP_FryingBar.BP_FryingBar_C"))
  (set `self.FryingBar` (`|GetArrayItem` _outactors)))

(event `self.ReceiveTick`
  (params (DeltaSeconds :type "Float (single-precision)"))
  (bind _widget (`/Game/BP_FryingBar.Widget` (`self.FryingBar`)))
  ;[1 1 1] If food i placed on pan: start timer and make food done when timer ends.
  (if (`self.HasFoodOnTop?`)
    (`SceneComponent.SetVisibility` _widget true false)
    (if (>= (`/Game/BP_FryingBar.Progress` (`self.FryingBar`)) 100.0)
      (bind _asbp_food (cast `/Game/FoodBP/BP_Food` (`self.Food`)))
      (`/Game/FoodBP/BP_Food.FoodDone` _asbp_food)
      (`KismetSystemLibrary.K2_ClearAndInvalidateTimerHandle` (stale _returnvalue))
      (else
        (`/Engine/EditorBlueprintResources/StandardMacros.DoOnce` false :!label _label
          (:`Completed`
            (bind _asbp_food_frying (cast `/Game/FoodBP/BP_Food_Frying` (`self.Food`)))
            (bind _preparationtime (`/Game/FoodBP/BP_Food_Frying.PreparationTime` _asbp_food_frying))
            (bind _foodprogress (`/Game/FoodBP/BP_Food_Frying.FoodProgress` _asbp_food_frying))
            (set `/Game/BP_FryingBar.Progress` (* (/ (- _preparationtime _foodprogress) _preparationtime) 100.0) (`self.FryingBar`))
            (bind _returnvalue (`KismetSystemLibrary.K2_SetTimer` null "Fry" (/ _preparationtime 20.0) true))
            ;;[1 1 1] Play sizzling sound when food is placed, for (preparation time) seconds.
            (`GameplayStatics.PlaySoundAtLocation` "/Game/Sound/soundPan.soundPan" (`self.K2_GetActorLocation` (`self.Food`)) (struct) 0.5 1.0 (- 24.5 _foodprogress))))))
    (else
      (`SceneComponent.SetVisibility` _widget false false)
      (`/Game/BP_FryingBar.ResetFryingBar` (`self.FryingBar`))
      (goto _label :!via `Reset`))))

(event `/Game/BPI_OutlineOnFood.SetOutlineOn`
  (params (Food :type "Actor Object Reference"))
  ;[1 1 1] Give pan green outline if food in hand can be placed on pan.
  (if (`KismetMathLibrary.ClassIsChildOf` (`GameplayStatics.GetObjectClass` Food) "/Game/FoodBP/BP_Food_Frying.BP_Food_Frying_C")
    (if (not (`self.HasFoodOnTop?`))
      (bind _asbp_food (cast `/Game/FoodBP/BP_Food` Food))
      (if (not (`/Game/FoodBP/BP_Food.Done` _asbp_food))
        (`PrimitiveComponent.SetRenderCustomDepth` (`self.Pan`) true)
        (set `self.OutlineOn` true)))))

(event `/Game/BPI_OutlineOff.SetOutlineOff`
  ;[1 1 1] Remove green outline when hand is not touching pan.
  (if (`self.OutlineOn`)
    (`PrimitiveComponent.SetRenderCustomDepth` (`self.Pan`) false)
    (set `self.OutlineOn` false)))

(event `/Game/BPI_InteractLeft.Interact`
  (bind _food (`self.Food`))
  ;[1 1 1] When player interacts with frying pan
  (if (`self.HasFoodOnTop?`)
    (bind _asfirst_person_character_1 (cast `/Game/FirstPersonBP/Blueprints/FirstPersonCharacter1` (`GameplayStatics.GetPlayerCharacter` 0)))
    (`/Engine/EditorBlueprintResources/StandardMacros.IsValid` _food
      (:`Is Valid`
        (bind _food_2 (`/Game/FirstPersonBP/Blueprints/FirstPersonCharacter1.Food` _asfirst_person_character_1))
        (`/Engine/EditorBlueprintResources/StandardMacros.IsValid` _food_2
          (:`Is Valid`
            (bind _asbp_food (cast `/Game/FoodBP/BP_Food` _food_2))
            (if (`/Game/FoodBP/BP_Food.Done` _asbp_food)
              _
              (elif (`KismetMathLibrary.ClassIsChildOf` (`GameplayStatics.GetObjectClass` _asbp_food) "/Game/FoodBP/BP_Food_Frying.BP_Food_Frying_C")
                (`self.K2_SetActorTransform` _asbp_food (`KismetMathLibrary.MakeTransform` (.location (`SceneComponent.K2_GetComponentToWorld` (`self.SnapPoint`))) (.rotation (`SceneComponent.K2_GetComponentToWorld` (`self.SnapPoint`)))) false false)
                (set `/Game/FirstPersonBP/Blueprints/FirstPersonCharacter1.Food` _food _asfirst_person_character_1)
                (set `/Game/FirstPersonBP/Blueprints/FirstPersonCharacter1.HoldingFood` true _asfirst_person_character_1)
                (set `self.Food` _asbp_food)
                (set `self.HasFoodOnTop?` true)
                (bind _asbp_food_frying (cast `/Game/FoodBP/BP_Food_Frying` (`self.Food`)))
                (bind _preparationtime (`/Game/FoodBP/BP_Food_Frying.PreparationTime` _asbp_food_frying))
                (set `/Game/BP_FryingBar.Progress` (* (/ (- _preparationtime (`/Game/FoodBP/BP_Food_Frying.FoodProgress` _asbp_food_frying)) _preparationtime) 100.0) (`self.FryingBar`))
                (goto _label :!via `Reset`))))
          (:`Is Not Valid`
            (set `/Game/FirstPersonBP/Blueprints/FirstPersonCharacter1.Food` _food _asfirst_person_character_1)
            (set `/Game/FirstPersonBP/Blueprints/FirstPersonCharacter1.HoldingFood` true _asfirst_person_character_1)
            (set `self.Food` null)
            (set `self.HasFoodOnTop?` false)))))
    (else
      (`self.DropFood`))))

(fn `DropFood`
  (bind _asfirst_person_character_1 (cast `/Game/FirstPersonBP/Blueprints/FirstPersonCharacter1` (`GameplayStatics.GetPlayerCharacter` 0)))
  (bind _asbp_food (cast `/Game/FoodBP/BP_Food` (`/Game/FirstPersonBP/Blueprints/FirstPersonCharacter1.Food` _asfirst_person_character_1)))
  (if (`/Game/FoodBP/BP_Food.Done` _asbp_food)
    _
    (elif (`KismetMathLibrary.ClassIsChildOf` (`GameplayStatics.GetObjectClass` _asbp_food) "/Game/FoodBP/BP_Food_Frying.BP_Food_Frying_C")
      (`self.K2_SetActorTransform` _asbp_food (`KismetMathLibrary.MakeTransform` (.location (`SceneComponent.K2_GetComponentToWorld` (`self.SnapPoint`))) (.rotation (`SceneComponent.K2_GetComponentToWorld` (`self.SnapPoint`)))) false false)
      (set `/Game/FirstPersonBP/Blueprints/FirstPersonCharacter1.Food` null _asfirst_person_character_1)
      (set `/Game/FirstPersonBP/Blueprints/FirstPersonCharacter1.HoldingFood` false _asfirst_person_character_1)
      (set `self.Food` _asbp_food)
      (set `self.HasFoodOnTop?` true))))

(fn `Fry`
  (`/Game/BP_FryingBar.increaseFryingBar` (`self.FryingBar`) 5.0)
  (bind _asbp_food_frying (cast `/Game/FoodBP/BP_Food_Frying` (`self.Food`)))
  (set `/Game/FoodBP/BP_Food_Frying.FoodProgress` (- (`/Game/FoodBP/BP_Food_Frying.FoodProgress` _asbp_food_frying) 1.0) _asbp_food_frying))

(fn `UserConstructionScript`)