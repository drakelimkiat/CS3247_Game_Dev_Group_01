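; Serving plate where the player assembles finished food into a burger, chicken rice or salad.
; Interact absorbs compatible held food into ingredient and dish flags, or, when empty-handed, spawns the matching food into the player's hands and clears the plate.
; Tick shows the pre-built mesh for the current combination and marks full dishes complete.
; Events toggle a custom-depth outline for placeable food and a tutorial arrow.
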(event `self.ReceiveBeginPlay`
  (`self.SetAllNotVisible`))

(event `/Game/BPI_InteractLeft.Interact`
  (bind _asfirst_person_character_1 (cast `/Game/FirstPersonBP/Blueprints/FirstPersonCharacter1` (`GameplayStatics.GetPlayerCharacter` 0)))
  (if (`/Game/FirstPersonBP/Blueprints/FirstPersonCharacter1.HoldingFood` _asfirst_person_character_1)
    (bind _asbp_food (cast `/Game/FoodBP/BP_Food` (`/Game/FirstPersonBP/Blueprints/FirstPersonCharacter1.Food` _asfirst_person_character_1)))
    (if (`/Game/FoodBP/BP_Food.Done` _asbp_food)
      (if (`KismetMathLibrary.ClassIsChildOf` (`GameplayStatics.GetObjectClass` _asbp_food) "/Game/FoodBP/BP_Food_BurgerMeat.BP_Food_BurgerMeat_C")
        (if (`self.HasPatty?`)
          _
          (elif (`self.IsEmpty`)
            (set `self.HasPatty?` true :!label _label)
            (set `self.IsBurger` true :!label _label_2)
            (set `self.IsEmpty` false :!label _label_3)
            (set `/Game/FirstPersonBP/Blueprints/FirstPersonCharacter1.Food` null _asfirst_person_character_1)
            (set `/Game/FirstPersonBP/Blueprints/FirstPersonCharacter1.HoldingFood` false _asfirst_person_character_1)
            (`self.K2_DestroyActor` _asbp_food)
            (elif (`self.IsBurger`)
              (goto _label))))
        (elif (`KismetMathLibrary.ClassIsChildOf` (`GameplayStatics.GetObjectClass` _asbp_food) "/Game/FoodBP/BP_Food_BurgerBun.BP_Food_BurgerBun_C")
          (if (`self.HasBun?`)
            _
            (elif (`self.IsEmpty`)
              (set `self.HasBun?` true :!label _label_4)
              (goto _label_2)
              (elif (`self.IsBurger`)
                (goto _label_4))))
          (elif (`KismetMathLibrary.ClassIsChildOf` (`GameplayStatics.GetObjectClass` _asbp_food) "/Game/FoodBP/BP_Food_Cheese.BP_Food_Cheese_C")
            (if (`self.HasCheese?`)
              _
              (elif (`self.IsEmpty`)
                (set `self.HasCheese?` true :!label _label_5)
                (goto _label_2)
                (elif (`self.IsBurger`)
                  (goto _label_5))))
            (elif (`KismetMathLibrary.ClassIsChildOf` (`GameplayStatics.GetObjectClass` _asbp_food) "/Game/FoodBP/BP_Food_Burger_Meat_Bun.BP_Food_Burger_Meat_Bun_C")
              (if (`self.IsEmpty`)
                (set `self.HasPatty?` true :!label _label_6)
                (set `self.HasBun?` true)
                (goto _label_2)
                (elif (and (`self.IsBurger`) (not (`self.HasPatty?`)) (not (`self.HasBun?`)) (`self.HasCheese?`))
                  (goto _label_6)))
              (elif (`KismetMathLibrary.ClassIsChildOf` (`GameplayStatics.GetObjectClass` _asbp_food) "/Game/FoodBP/BP_Food_Burger_Meat_Cheese.BP_Food_Burger_Meat_Cheese_C")
                (if (`self.IsEmpty`)
                  (set `self.HasPatty?` true :!label _label_7)
                  (set `self.HasCheese?` true)
                  (goto _label_2)
                  (elif (and (`self.IsBurger`) (not (`self.HasPatty?`)) (`self.HasBun?`) (not (`self.HasCheese?`)))
                    (goto _label_7)))
                (elif (`KismetMathLibrary.ClassIsChildOf` (`GameplayStatics.GetObjectClass` _asbp_food) "/Game/FoodBP/BP_Burger_Cheese_Bun.BP_Burger_Cheese_Bun_C")
                  (if (`self.IsEmpty`)
                    (set `self.HasBun?` true :!label _label_8)
                    (set `self.HasCheese?` true)
                    (goto _label_2)
                    (elif (and (`self.IsBurger`) (`self.HasPatty?`) (not (`self.HasBun?`)) (not (`self.HasCheese?`)))
                      (goto _label_8)))
                  (elif (`KismetMathLibrary.ClassIsChildOf` (`GameplayStatics.GetObjectClass` _asbp_food) "/Game/FoodBP/BP_Food_Burger.BP_Food_Burger_C")
                    (if (`self.IsEmpty`)
                      (set `self.HasPatty?` true)
                      (set `self.HasBun?` true)
                      (set `self.HasCheese?` true)
                      (goto _label_2))
                    (elif (`KismetMathLibrary.ClassIsChildOf` (`GameplayStatics.GetObjectClass` _asbp_food) "/Game/FoodBP/BP_Food_Rice.BP_Food_Rice_C")
                      (if (`self.HasRice?`)
                        _
                        (elif (`self.IsEmpty`)
                          (set `self.HasRice?` true :!label _label_9)
                          (set `self.IsChickenRice` true :!label _label_10)
                          (goto _label_3)
                          (elif (`self.IsChickenRice`)
                            (goto _label_9))))
                      (elif (`KismetMathLibrary.ClassIsChildOf` (`GameplayStatics.GetObjectClass` _asbp_food) "/Game/FoodBP/BP_Food_Chicken.BP_Food_Chicken_C")
                        (if (`self.HasChicken?`)
                          _
                          (elif (`self.IsEmpty`)
                            (set `self.HasChicken?` true :!label _label_11)
                            (goto _label_10)
                            (elif (`self.IsChickenRice`)
                              (goto _label_11))))
                        (elif (`KismetMathLibrary.ClassIsChildOf` (`GameplayStatics.GetObjectClass` _asbp_food) "/Game/FoodBP/BP_Food_ChickenRice.BP_Food_ChickenRice_C")
                          (if (`self.IsEmpty`)
                            (set `self.HasRice?` true)
                            (set `self.HasChicken?` true)
                            (goto _label_10))
                          (elif (`KismetMathLibrary.ClassIsChildOf` (`GameplayStatics.GetObjectClass` _asbp_food) "/Game/FoodBP/BP_Food_Lettuce.BP_Food_Lettuce_C")
                            (if (`self.HasLettuce?`)
                              _
                              (elif (`self.IsEmpty`)
                                (set `self.HasLettuce?` true :!label _label_12)
                                (set `self.IsSalad` true :!label _label_13)
                                (goto _label_3)
                                (elif (`self.IsSalad`)
                                  (goto _label_12))))
                            (elif (`KismetMathLibrary.ClassIsChildOf` (`GameplayStatics.GetObjectClass` _asbp_food) "/Game/FoodBP/BP_Food_Carrot.BP_Food_Carrot_C")
                              (if (`self.HasCarrots?`)
                                _
                                (elif (`self.IsEmpty`)
                                  (set `self.HasCarrots?` true :!label _label_14)
                                  (goto _label_13)
                                  (elif (`self.IsSalad`)
                                    (goto _label_14))))
                              (elif (`KismetMathLibrary.ClassIsChildOf` (`GameplayStatics.GetObjectClass` _asbp_food) "/Game/FoodBP/BP_Food_Salad.BP_Food_Salad_C")
                                (if (`self.IsEmpty`)
                                  (set `self.HasLettuce?` true)
                                  (set `self.HasCarrots?` true)
                                  (goto _label_13)))))))))))))))
      (else
        (`KismetSystemLibrary.PrintString` "not done")))
    (else
      (`self.SpawnFood`))))

(event `self.ReceiveTick`
  (params (DeltaSeconds :type "Float (single-precision)"))
  (bind _hasrice_ (`self.HasRice?`))
  (bind _haschicken_ (`self.HasChicken?`))
  (bind _haslettuce_ (`self.HasLettuce?`))
  (bind _hascarrots_ (`self.HasCarrots?`))
  (bind _haspatty_ (`self.HasPatty?`))
  (bind _hasbun_ (`self.HasBun?`))
  (bind _hascheese_ (`self.HasCheese?`))
  (if (`self.IsEmpty`)
    (`self.SetAllNotVisible`)
    (elif (`self.IsBurger`)
      (if (and _haspatty_ _hasbun_ _hascheese_)
        (`self.SetAllNotVisible`)
        (`SceneComponent.SetVisibility` (`self.Burger_Complete`) true false)
        (set `self.IsComplete` true :!label _label_15)
        (elif (and _haspatty_ _hasbun_)
          (`self.SetAllNotVisible`)
          (`SceneComponent.SetVisibility` (`self.Burger_PattyBun`) true false)
          (elif (and _haspatty_ _hascheese_)
            (`self.SetAllNotVisible`)
            (`SceneComponent.SetVisibility` (`self.Burger_PattyCheese`) true false)
            (elif (and _hasbun_ _hascheese_)
              (`self.SetAllNotVisible`)
              (`SceneComponent.SetVisibility` (`self.Burger_BunCheese`) true false)
              (elif _haspatty_
                (`self.SetAllNotVisible`)
                (`SceneComponent.SetVisibility` (`self.Burger_Patty`) true false)
                (elif _hasbun_
                  (`self.SetAllNotVisible`)
                  (`SceneComponent.SetVisibility` (`self.Burger_Bun`) true false)
                  (elif _hascheese_
                    (`self.SetAllNotVisible`)
                    (`SceneComponent.SetVisibility` (`self.Burger_Cheese`) true false))))))))
      (elif (`self.IsChickenRice`)
        (if (and _hasrice_ _haschicken_)
          (`self.SetAllNotVisible`)
          (`SceneComponent.SetVisibility` (`self.ChickenRice_Complete`) true false)
          (goto _label_15)
          (elif _hasrice_
            (`self.SetAllNotVisible`)
            (`SceneComponent.SetVisibility` (`self.ChickenRice_Rice`) true false)
            (elif _haschicken_
              (`self.SetAllNotVisible`)
              (`SceneComponent.SetVisibility` (`self.ChickenRice_Chicken`) true false))))
        (elif (`self.IsSalad`)
          (if (and _haslettuce_ _hascarrots_)
            (`self.SetAllNotVisible`)
            (`SceneComponent.SetVisibility` (`self.Salad_Complete`) true false)
            (goto _label_15)
            (elif _haslettuce_
              (`self.SetAllNotVisible`)
              (`SceneComponent.SetVisibility` (`self.Salad_Lettuce`) true false)
              (elif _hascarrots_
                (`self.SetAllNotVisible`)
                (`SceneComponent.SetVisibility` (`self.Salad_Carrots`) true false)))))))))

(event `/Game/BPI_TutorialIndicatorOn.SetTutorialIndicatorOn`
  ;[1 1 1] Tutorial: Arrow on/off
  (`/Engine/EditorBlueprintResources/StandardMacros.IsValid` (`self.Arrow`)
    (:`Is Not Valid`
      (bind _returnvalue (`|SpawnActorFromClass` "/Game/BP_TutorialArrow.BP_TutorialArrow_C" (`KismetMathLibrary.MakeTransform` (+ (`SceneComponent.K2_GetComponentLocation` (`self.SnapPoint`)) (0.0 0.0 25.0)) (struct :`Yaw` 220.0)) "Undefined" "OverrideRootScale" null null))
      (set `self.Arrow` _returnvalue))))

(event `/Game/BPI_TutorialIndicatorOff.SetTutorialIndicatorOff`
  (bind _arrow (`self.Arrow`))
  ;[1 1 1] Tutorial: Arrow on/off
  (`/Engine/EditorBlueprintResources/StandardMacros.IsValid` _arrow
    (:`Is Valid`
      (`self.K2_DestroyActor` _arrow))))

(event `/Game/BPI_OutlineOnFood.SetOutlineOn`
  (params (Food :type "Actor Object Reference"))
  (bind _returnvalue (`GameplayStatics.GetObjectClass` Food))
  (bind _returnvalue_2 (`GameplayStatics.GetObjectClass` Food))
  (bind _returnvalue_3 (`GameplayStatics.GetObjectClass` Food))
  ;[1 1 1] Outline on/off if food can be placed
  (bind _asbp_food (cast `/Game/FoodBP/BP_Food` Food))
  (if (`/Game/FoodBP/BP_Food.Done` _asbp_food)
    (if (`self.IsEmpty`)
      (`PrimitiveComponent.SetRenderCustomDepth` (`self.Plate`) true)
      (elif (`self.IsComplete`)
        _
        (elif (`self.IsBurger`)
          (if (`self.HasCheese?`)
            (if (`self.HasBun?`) :!label _label_16
              (if (`self.HasPatty?`) :!label _label_17
                _
                (elif (== _returnvalue "/Game/FoodBP/BP_Food_BurgerMeat.BP_Food_BurgerMeat_C")
                  (`PrimitiveComponent.SetRenderCustomDepth` (`self.Plate`) true :!label _label_18)))
              (elif (== _returnvalue "/Game/FoodBP/BP_Food_BurgerBun.BP_Food_BurgerBun_C")
                (goto _label_18)
                (else
                  (goto _label_17))))
            (elif (== _returnvalue "/Game/FoodBP/BP_Food_Cheese.BP_Food_Cheese_C")
              (goto _label_18)
              (else
                (goto _label_16))))
          (elif (`self.IsSalad`)
            (if (`self.HasLettuce?`)
              (if (== _returnvalue_2 "/Game/BP_ChoppingBoard.BP_ChoppingBoard_C")
                (`PrimitiveComponent.SetRenderCustomDepth` (`self.Plate`) true :!label _label_19))
              (elif (== _returnvalue_2 "/Game/FoodBP/BP_Food_Lettuce.BP_Food_Lettuce_C")
                (goto _label_19)))
            (elif (`self.IsChickenRice`)
              (if (`self.HasChicken?`)
                (if (== _returnvalue_3 "/Game/FoodBP/BP_Food_Rice.BP_Food_Rice_C")
                  (`PrimitiveComponent.SetRenderCustomDepth` (`self.Plate`) true :!label _label_20))
                (elif (== _returnvalue_3 "/Game/FoodBP/BP_Food_Chicken.BP_Food_Chicken_C")
                  (goto _label_20))))))))))

(event `/Game/BPI_OutlineOff.SetOutlineOff`
  ;[1 1 1] Outline on/off if food can be placed
  (`PrimitiveComponent.SetRenderCustomDepth` (`self.Plate`) false))

(fn `AddAllToArray`
  (`KismetArrayLibrary.Array_Add` (`self.FoodMeshes`) (`self.Burger_Complete`))
  (`KismetArrayLibrary.Array_Add` (`self.FoodMeshes`) (`self.Burger_Patty`))
  (`KismetArrayLibrary.Array_Add` (`self.FoodMeshes`) (`self.Burger_Bun`))
  (`KismetArrayLibrary.Array_Add` (`self.FoodMeshes`) (`self.Burger_Cheese`))
  (`KismetArrayLibrary.Array_Add` (`self.FoodMeshes`) (`self.Burger_PattyBun`))
  (`KismetArrayLibrary.Array_Add` (`self.FoodMeshes`) (`self.Burger_PattyCheese`))
  (`KismetArrayLibrary.Array_Add` (`self.FoodMeshes`) (`self.Burger_BunCheese`))
  (`KismetArrayLibrary.Array_Add` (`self.FoodMeshes`) (`self.ChickenRice_Complete`))
  (`KismetArrayLibrary.Array_Add` (`self.FoodMeshes`) (`self.ChickenRice_Rice`))
  (`KismetArrayLibrary.Array_Add` (`self.FoodMeshes`) (`self.ChickenRice_Chicken`))
  (`KismetArrayLibrary.Array_Add` (`self.FoodMeshes`) (`self.Salad_Complete`))
  (`KismetArrayLibrary.Array_Add` (`self.FoodMeshes`) (`self.Salad_Lettuce`))
  (`KismetArrayLibrary.Array_Add` (`self.FoodMeshes`) (`self.Salad_Carrots`)))

(fn `SetAllNotVisible`
  (for _array_element (`self.FoodMeshes`)
    (`SceneComponent.SetVisibility` _array_element false false)))

(fn `SetEmpty`
  (set `self.HasPatty?` false)
  (set `self.HasBun?` false)
  (set `self.HasCheese?` false)
  (set `self.HasRice?` false)
  (set `self.HasChicken?` false)
  (set `self.HasLettuce?` false)
  (set `self.HasPatty?` false)
  (set `self.HasCarrots?` false)
  (set `self.HasTomatoes?` false)
  (set `self.IsBurger` false)
  (set `self.IsChickenRice` false)
  (set `self.IsSalad` false)
  (set `self.IsComplete` false)
  (set `self.IsEmpty` true))

(fn `SpawnFood`
  (bind _hasrice_ (`self.HasRice?`))
  (bind _haschicken_ (`self.HasChicken?`))
  (bind _haslettuce_ (`self.HasLettuce?`))
  (bind _hascarrots_ (`self.HasCarrots?`))
  (bind _haspatty_ (`self.HasPatty?`))
  (bind _hasbun_ (`self.HasBun?`))
  (bind _hascheese_ (`self.HasCheese?`))
  (if (`self.IsBurger`)
    (if (and _haspatty_ _hasbun_ _hascheese_)
      (set `self.SpawnClass` "/Game/FoodBP/BP_Food_Burger.BP_Food_Burger_C")
      (bind _returnvalue (`|SpawnActorFromClass` (`self.SpawnClass`) (`KismetMathLibrary.MakeTransform` (0.0 0.0 0.0)) "Undefined" "OverrideRootScale" null null :!label _label))
      (if (not (`KismetMathLibrary.ClassIsChildOf` (`GameplayStatics.GetObjectClass` _returnvalue) "/Game/FoodBP/BP_Food_NoPrep.BP_Food_NoPrep_C"))
        (bind _asbp_food (cast `/Game/FoodBP/BP_Food` _returnvalue))
        (`/Game/FoodBP/BP_Food.FoodDone` _asbp_food))
      (bind _asfirst_person_character_1 (cast `/Game/FirstPersonBP/Blueprints/FirstPersonCharacter1` (`GameplayStatics.GetPlayerCharacter` 0)))
      (set `/Game/FirstPersonBP/Blueprints/FirstPersonCharacter1.Food` _returnvalue _asfirst_person_character_1)
      (set `/Game/FirstPersonBP/Blueprints/FirstPersonCharacter1.HoldingFood` true _asfirst_person_character_1)
      (`self.SetEmpty`)
      (elif (and _haspatty_ _hasbun_)
        (set `self.SpawnClass` "/Game/FoodBP/BP_Food_Burger_Meat_Bun.BP_Food_Burger_Meat_Bun_C")
        (goto _label)
        (elif (and _haspatty_ _hascheese_)
          (set `self.SpawnClass` "/Game/FoodBP/BP_Food_Burger_Meat_Cheese.BP_Food_Burger_Meat_Cheese_C")
          (goto _label)
          (elif (and _hasbun_ _hascheese_)
            (set `self.SpawnClass` "/Game/FoodBP/BP_Burger_Cheese_Bun.BP_Burger_Cheese_Bun_C")
            (goto _label)
            (elif _haspatty_
              (set `self.SpawnClass` "/Game/FoodBP/BP_Food_BurgerMeat.BP_Food_BurgerMeat_C")
              (goto _label)
              (elif _hasbun_
                (set `self.SpawnClass` "/Game/FoodBP/BP_Food_BurgerBun.BP_Food_BurgerBun_C")
                (goto _label)
                (elif _hascheese_
                  (set `self.SpawnClass` "/Game/FoodBP/BP_Food_Cheese.BP_Food_Cheese_C")
                  (goto _label))))))))
    (elif (`self.IsChickenRice`)
      (if (and _hasrice_ _haschicken_)
        (set `self.SpawnClass` "/Game/FoodBP/BP_Food_ChickenRice.BP_Food_ChickenRice_C")
        (goto _label)
        (elif _hasrice_
          (set `self.SpawnClass` "/Game/FoodBP/BP_Food_Rice.BP_Food_Rice_C")
          (goto _label)
          (elif _haschicken_
            (set `self.SpawnClass` "/Game/FoodBP/BP_Food_Chicken.BP_Food_Chicken_C")
            (goto _label))))
      (elif (`self.IsSalad`)
        (if (and _haslettuce_ _hascarrots_)
          (set `self.SpawnClass` "/Game/FoodBP/BP_Food_Salad.BP_Food_Salad_C")
          (goto _label)
          (elif _haslettuce_
            (set `self.SpawnClass` "/Game/FoodBP/BP_Food_Lettuce.BP_Food_Lettuce_C")
            (goto _label)
            (elif _hascarrots_
              (set `self.SpawnClass` "/Game/FoodBP/BP_Food_Carrot.BP_Food_Carrot_C")
              (goto _label))))))))

(fn `UserConstructionScript`
  (`self.AddAllToArray`))