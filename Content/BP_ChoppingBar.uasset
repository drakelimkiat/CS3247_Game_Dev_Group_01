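; BP_ChoppingBar is a Blueprint that displays chopping progress as a progress bar on a widget component.
; Each Tick it casts the component's user widget to ChoppingBar and sets ProgressBar18 to Progress scaled from a 0–100 range.
; IncreaseChoppingBar is the function for raising Progress, and ResetChoppingBar sets it back to zero.
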(event `self.ReceiveTick`
  (params (DeltaSeconds :type "Float (single-precision)"))
  (bind _aschopping_bar (cast `/Game/ChoppingBar` (`WidgetComponent.GetUserWidgetObject` (`self.Widget`))))
  (`ProgressBar.SetPercent` (`/Game/ChoppingBar.ProgressBar_18` _aschopping_bar) (/ (`self.Progress`) 100.0)))

(fn `IncreaseChoppingBar`
  (params (Progress :type "Float (double-precision)"))
  (set `self.Progress` (+ Progress (`self.Progress`))))

(fn `ResetChoppingBar`
  (set `self.Progress` 0.0))

(fn `UserConstructionScript`)