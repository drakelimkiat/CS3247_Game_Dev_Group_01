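; BP_Pan1 is a frying pan that cooks BP_Food_Frying items overlapping its collision box.
; On overlap it stores the food and starts a looping Fry timer that adds 5% per step to the level's first BP_FryingBar, spreading the fill over PreparationTime.
; Tick shows the bar while food is flagged, calls FoodDone and clears the timer at 100, otherwise hides and resets it.
; Nothing here clears the food flag.
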(event `self.ReceiveBeginPlay`
  (bind _outactors (`GameplayStatics.GetAllActorsOfClass` "/Game/BP_FryingBar.BP_FryingBar_C"))
  (set `self.FryingBar` (`|GetArrayItem` _outactors)))

(event `self.ReceiveTick`
  (params (DeltaSeconds :type "Float (single-precision)"))
  (bind _widget (`/Game/BP_FryingBar.Widget` (`self.FryingBar`)))
  (if (`self.HasFoodOnTop?`)
    (`SceneComponent.SetVisibility` _widget true false)
    (if (>= (`/Game/BP_FryingBar.Progress` (`self.FryingBar`)) 100.0)
      (bind _asbp_food_frying (cast `/Game/FoodBP/BP_Food_Frying` (`self.Food`)))
      (`/Game/FoodBP/BP_Food_Frying.FoodDone` _asbp_food_frying)
      (`KismetSystemLibrary.K2_ClearAndInvalidateTimerHandle` (stale `self.CollisionBox.OnComponentBeginOverlap` _returnvalue)))
    (else
      (`SceneComponent.SetVisibility` _widget false false)
      (`/Game/BP_FryingBar.ResetFryingBar` (`self.FryingBar`)))))

(event `self.CollisionBox.OnComponentBeginOverlap`
  (params (OverlappedComponent :type "PrimitiveComponent Object Reference") (OtherActor :type "Actor Object Reference") (OtherComp :type "PrimitiveComponent Object Reference") (OtherBodyIndex :type Integer) (bFromSweep :type Boolean) (SweepResult :type "HitResult Structure (by ref)"))
  (if (`KismetMathLibrary.ClassIsChildOf` (`GameplayStatics.GetObjectClass` OtherActor) "/Game/FoodBP/BP_Food_Frying.BP_Food_Frying_C")
    (set `self.HasFoodOnTop?` true)
    (bind _output_get (set `self.Food` OtherActor))
    (bind _asbp_food_frying (cast `/Game/FoodBP/BP_Food_Frying` _output_get))
    (bind _returnvalue (`KismetSystemLibrary.K2_SetTimer` null "Fry" (/ (`/Game/FoodBP/BP_Food_Frying.PreparationTime` _asbp_food_frying) 20.0) true))))

(fn `Fry`
  (`/Game/BP_FryingBar.increaseFryingBar` (`self.FryingBar`) 5.0))

(fn `UserConstructionScript`)