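; BP_Food_Projectile is a food projectile that raises the satisfaction of whatever it hits.
; On hit it sends a fixed ChangeSatisfaction interface message to the other actor and destroys itself, with the physics impulse logic left disconnected.
; The construction script applies FoodMesh and FoodMeshScale to the Food component through LoadGunWithMesh, falling back to an unscaled burger when no valid mesh is set.
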(event `self.ReceiveHit`
  (params (MyComp :type "PrimitiveComponent Object Reference") (Other :type "Actor Object Reference") (OtherComp :type "PrimitiveComponent Object Reference") (bSelfMoved :type Boolean) (HitLocation :type "Vector Structure") (HitNormal :type "Vector Structure") (NormalImpulse :type "Vector Structure") (Hit :type "HitResult Structure (by ref)"))
  ;[1 1 1] Call ChangeSatisfaction to any physics object we hit (physics impulse disabled so no bounce occurs)
  (message `/Game/ChangeSatisfaction.ChangeSatisfaction` Other 25.0)
  (`self.K2_DestroyActor`) ; Then destroy this projectile
)

(fn `LoadGunWithMesh`
  (params (FoodMesh :type "StaticMesh Object Reference"))
  (`StaticMeshComponent.SetStaticMesh` (`self.Food`) FoodMesh))

(fn `UserConstructionScript`
  (bind _foodmesh (`self.FoodMesh`))
  (`/Engine/EditorBlueprintResources/StandardMacros.IsValid` _foodmesh
    (:`Is Valid`
      _)
    (:`Is Not Valid`
      (set `self.FoodMesh` "/Game/Assets/Burger/Burger.Burger")
      (set `self.FoodMeshScale` (1.0 1.0 1.0))))
  (`self.LoadGunWithMesh` _foodmesh)
  (`SceneComponent.SetWorldScale3D` (`self.Food`) (`self.FoodMeshScale`)))