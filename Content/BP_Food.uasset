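; BP_Food is a food actor that tracks chopping progress when something overlaps it.
; On BeginPlay it caches the first BP_ChoppingBar found in the level.
; Each overlap calls Interact with a fixed step, which adds that step to the bar's Progress and stores the capped result in Progress.
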(event `self.ReceiveBeginPlay`
  (bind _outactors (`GameplayStatics.GetAllActorsOfClass` "/Game/BP_ChoppingBar.BP_ChoppingBar_C"))
  (set `self.ChoppingBar` (`|GetArrayItem` _outactors)))

(event `self.ReceiveActorBeginOverlap`
  (params (OtherActor :type "Actor Object Reference"))
  (`self.Interact` 1.0))

(fn `Interact`
  (params (Progress :type "Float (double-precision)"))
  (returns (something :type "Float (double-precision)"))
  (bind _returnvalue (+ Progress (`/Game/BP_ChoppingBar.Progress` (`self.ChoppingBar`))))
  (if (>= _returnvalue 100.0)
    (set `self.Progress` 100.0)
    (else
      (set `self.Progress` _returnvalue))))

(fn `UserConstructionScript`)