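; BP_TV is an in-world TV that switches between an image screen, a complaints score display and a game-over display by toggling component visibility.
; SetImage shows the Screen, passes the image to its HUD_TV widget and can flag an automatic switch back.
; Tick consumes that flag and restores the score screen after a five-second delay.
; SetGameOver reveals the game-over display and hides the score.
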(event `self.ReceiveTick`
  (params (DeltaSeconds :type "Float (single-precision)"))
  (if (`self.SwitchBack`)
    (set `self.SwitchBack` false)
    (`KismetSystemLibrary.Delay` 5.0)
    (`self.SetScoreScreen`)))

(fn `SetGameOver`
  (`SceneComponent.SetVisibility` (`self.GameOver`) true false)
  (`SceneComponent.SetVisibility` (`self.Complaints&ScoreHUD`) false false))

(fn `SetImage`
  (params (Image :type Integer) (SwitchBack :type Boolean))
  (`SceneComponent.SetVisibility` (`self.Complaints&ScoreHUD`) false false)
  (`SceneComponent.SetVisibility` (`self.Screen`) true false)
  (bind _ashud_tv (cast `/Game/HUD_TV` (`WidgetComponent.GetUserWidgetObject` (`self.Screen`))))
  (`/Game/HUD_TV.SetImage` _ashud_tv Image)
  (set `self.SwitchBack` SwitchBack))

(fn `SetScoreScreen`
  (`SceneComponent.SetVisibility` (`self.Screen`) false false)
  (`SceneComponent.SetVisibility` (`self.Complaints&ScoreHUD`) true false))

(fn `UserConstructionScript`)