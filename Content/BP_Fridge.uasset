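; BP_Fridge is an interactable fridge whose door toggles open and closed on Interact.
; OpenRotation and CloseRotation timelines swing Door and Box through 90 degrees of absolute world yaw, updating DoorOpen as they play.
; The open sound plays as the swing starts, and the quieter close sound when it finishes.
; BeginFocus and EndFocus toggle custom depth rendering on the Door.
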(event `self.ReceiveBeginPlay`)

(event `/Game/BPI_InteractLeft.Interact`
  ;[1 1 1] Close/Open door on interact left hand
  (if (`self.DoorOpen`)
    (`self.CloseDoor`)
    (else
      (`self.OpenDoor`))))

(event `OpenDoor`
  ;[1 1 1] Open door
  (`GameplayStatics.PlaySoundAtLocation` "/Game/Sound/fridgeOpen.fridgeOpen" (`SceneComponent.K2_GetComponentLocation` (`self.Body`)))
  (bind (_direction _0to90) (`Timeline|OpenRotation` :!via `PlayFromStart`)
    (:`Update`
      (`SceneComponent.K2_SetWorldRotation` (`self.Door`) (`KismetMathLibrary.MakeRotator` 0.0 0.0 _0to90) false false)
      (`SceneComponent.K2_SetWorldRotation` (`self.Box`) (`KismetMathLibrary.MakeRotator` 0.0 0.0 _0to90) false false)
      (set `self.DoorOpen` true))))

(event `CloseDoor`
  ;[1 1 1] Close door
  (bind (_direction _90to0) (`Timeline|CloseRotation` :!via `PlayFromStart`)
    (:`Update`
      (`SceneComponent.K2_SetWorldRotation` (`self.Door`) (`KismetMathLibrary.MakeRotator` 0.0 0.0 _90to0) false false)
      (`SceneComponent.K2_SetWorldRotation` (`self.Box`) (`KismetMathLibrary.MakeRotator` 0.0 0.0 _90to0) false false)
      (set `self.DoorOpen` false))
    (:`Finished`
      (`GameplayStatics.PlaySoundAtLocation` "/Game/Sound/fridgeClose.fridgeClose" (`SceneComponent.K2_GetComponentLocation` (`self.Body`)) (struct) 0.6))))

(fn `BeginFocus`
  (`PrimitiveComponent.SetRenderCustomDepth` (`self.Door`) true))

(fn `EndFocus`
  (`PrimitiveComponent.SetRenderCustomDepth` (`self.Door`) false))

(fn `UserConstructionScript`)