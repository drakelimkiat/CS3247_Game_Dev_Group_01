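; BP_EnemyKid is a kid enemy Blueprint that extends a parent class and has a satisfaction bar and a fade-out effect.
; On BeginPlay it creates a dynamic material instance for each body-part slot on its mesh.
; FadeOutMesh hides the satisfaction bar and plays a timeline that drives the FadeOut parameter on all those materials.
; Every Tick reapplies a fixed walk speed and calls DecreaseScore with the frame time before running parent logic.
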(event `self.ReceiveBeginPlay`
  (bind _mesh (`self.Mesh`))
  (`parent.ReceiveBeginPlay`)
  (bind _returnvalue (`PrimitiveComponent.CreateDynamicMaterialInstance` _mesh 0 "/Game/Character/Materials/M_EnemyKid_Arm.M_EnemyKid_Arm"))
  (bind _returnvalue_2 (`PrimitiveComponent.CreateDynamicMaterialInstance` _mesh 1 "/Game/Character/Materials/M_EnemyKid_Head.M_EnemyKid_Head"))
  (bind _returnvalue_3 (`PrimitiveComponent.CreateDynamicMaterialInstance` _mesh 2 "/Game/Character/Materials/M_EnemyKid_Initial.M_EnemyKid_Initial"))
  (bind _returnvalue_4 (`PrimitiveComponent.CreateDynamicMaterialInstance` _mesh 3 "/Game/Character/Materials/M_EnemyKid_Leg.M_EnemyKid_Leg"))
  (bind _returnvalue_5 (`PrimitiveComponent.CreateDynamicMaterialInstance` _mesh 4 "/Game/Character/Materials/M_EnemyKid_Shirt.M_EnemyKid_Shirt"))
  (bind _returnvalue_6 (`PrimitiveComponent.CreateDynamicMaterialInstance` _mesh 5 "/Game/Character/Materials/M_EnemyKid_Shorts.M_EnemyKid_Shorts"))
  (bind _returnvalue_7 (`PrimitiveComponent.CreateDynamicMaterialInstance` _mesh 6 "/Game/Character/Materials/M_EnemyKid_Torso.M_EnemyKid_Torso")))

(event `self.FadeOutMesh`
  (`SceneComponent.SetVisibility` (`self.SatisfactionBar`) false false)
  (bind (_direction _fade) (`Timeline|FadeOut`)
    (:`Update`
      (`MaterialInstanceDynamic.SetScalarParameterValue` (stale `self.ReceiveBeginPlay` _returnvalue) "FadeOut" _fade)
      (`MaterialInstanceDynamic.SetScalarParameterValue` (stale `self.ReceiveBeginPlay` _returnvalue_2) "FadeOut" _fade)
      (`MaterialInstanceDynamic.SetScalarParameterValue` (stale `self.ReceiveBeginPlay` _returnvalue_3) "FadeOut" _fade)
      (`MaterialInstanceDynamic.SetScalarParameterValue` (stale `self.ReceiveBeginPlay` _returnvalue_4) "FadeOut" _fade)
      (`MaterialInstanceDynamic.SetScalarParameterValue` (stale `self.ReceiveBeginPlay` _returnvalue_5) "FadeOut" _fade)
      (`MaterialInstanceDynamic.SetScalarParameterValue` (stale `self.ReceiveBeginPlay` _returnvalue_6) "FadeOut" _fade)
      (`MaterialInstanceDynamic.SetScalarParameterValue` (stale `self.ReceiveBeginPlay` _returnvalue_7) "FadeOut" _fade))))

(event `self.ReceiveTick`
  (params (DeltaSeconds :type "Float (single-precision)"))
  (`self.SetMaxWalkSpeed` 50.0)
  (`self.DecreaseScore` DeltaSeconds)
  (`parent.ReceiveTick` DeltaSeconds))

(fn `UserConstructionScript`)