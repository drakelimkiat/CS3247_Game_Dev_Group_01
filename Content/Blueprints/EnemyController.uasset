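; AI controller for an enemy that heads for a door and counter, counting as a complaint when its run ends.
; On BeginPlay it converts the pawn's yaw into an angle, buckets it by door count to select hard-coded door and counter positions, and writes them to EnemyBlackboard.
; Tick polls the blackboard's Ended flag, then adds complaints through RoundManager, decrements the player's enemy count and destroys the pawn.
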(event `self.ReceiveBeginPlay`
  (bind _returnvalue (`AIBlueprintHelperLibrary.GetBlackboard` self))
  (`self.UseBlackboard` (`self.EnemyBlackboard`))
  (`KismetSystemLibrary.Delay` 0.2)
  (`self.SetEnemyAngle`)
  (`self.SetLocationDoorValue`)
  (`self.SetLocationCounterValue`)
  (`BlackboardComponent.SetValueAsVector` _returnvalue (`self.LocationDoorKey`) (`self.LocationDoorValue`))
  (`BlackboardComponent.SetValueAsVector` _returnvalue (`self.LocationCounterKey`) (`self.LocationCounterValue`))
  (`BlackboardComponent.SetValueAsBool` _returnvalue (`self.EndedKey`) false)
  (`self.SetRoundManager`))

(event `self.ReceiveTick`
  (params (DeltaSeconds :type "Float (single-precision)"))
  (if (`BlackboardComponent.GetValueAsBool` (`AIBlueprintHelperLibrary.GetBlackboard` self) (`self.EndedKey`))
    (`/Game/Blueprints/RoundManager.AddComplaints` (`self.RoundManager`))
    (bind _asfirst_person_character_1 (cast `/Game/FirstPersonBP/Blueprints/FirstPersonCharacter1` (`GameplayStatics.GetPlayerCharacter` 0)))
    (`/Engine/EditorBlueprintResources/StandardMacros.DecrementInt` (`/Game/FirstPersonBP/Blueprints/FirstPersonCharacter1.NrOfEnimies` _asfirst_person_character_1)
      (:`  `
        (`self.K2_DestroyActor` (`self.K2_GetPawn`))))))

(fn `SetEnemyAngle`
  (bind (_returnvalue_roll _returnvalue_pitch _returnvalue_yaw) (`KismetMathLibrary.BreakRotator` (`self.K2_GetActorRotation` (`self.K2_GetPawn`))))
  (if (>= _returnvalue_yaw 0.0)
    (set `self.EnemyAngle` (* (+ _returnvalue_yaw -270.0) -1.0))
    (else
      (set `self.EnemyAngle` (* (+ _returnvalue_yaw 90.0) -1.0)))))

(fn `SetLocationCounterValue`
  (bind _returnvalue (`KismetMathLibrary.MakeVector` -410.0 -210.0))
  (set `self.LocationCounterValue` (select `int` (`KismetMathLibrary.FTrunc` (/ (`self.EnemyAngle`) (/ 180.0 (`KismetMathLibrary.Conv_IntToDouble` (`self.NumOfDoors`))))) :`0` (`KismetMathLibrary.MakeVector` -485.0 225.0) :`1` (`KismetMathLibrary.MakeVector` -410.0 210.0) :`2` (`KismetMathLibrary.MakeVector` -345.0 170.0) :`3` (`KismetMathLibrary.MakeVector` -295.0 115.0) :`4` (`KismetMathLibrary.MakeVector` -260.0 40.0) :`5` (`KismetMathLibrary.MakeVector` -260.0 -40.0) :`6` (`KismetMathLibrary.MakeVector` -295.0 -115.0) :`7` (`KismetMathLibrary.MakeVector` -345.0 -170.0) :`8` _returnvalue :`9` _returnvalue :`10` _returnvalue)))

(fn `SetLocationDoorValue`
  (bind _returnvalue (`KismetMathLibrary.MakeVector` -195.0 -725.0))
  (set `self.LocationDoorValue` (select `int` (`KismetMathLibrary.FTrunc` (/ (`self.EnemyAngle`) (/ 180.0 (`KismetMathLibrary.Conv_IntToDouble` (`self.NumOfDoors`))))) :`0` (`KismetMathLibrary.MakeVector` -15.0 695.0) :`1` (`KismetMathLibrary.MakeVector` 190.0 600.0) :`2` (`KismetMathLibrary.MakeVector` 350.0 440.0) :`3` (`KismetMathLibrary.MakeVector` 460.0 245.0) :`4` (`KismetMathLibrary.MakeVector` 500.0 25.0) :`5` (`KismetMathLibrary.MakeVector` 475.0 -205.0) :`6` (`KismetMathLibrary.MakeVector` 380.0 -410.0) :`7` (`KismetMathLibrary.MakeVector` 220.0 -575.0) :`8` (`KismetMathLibrary.MakeVector` 20.0 -685.0) :`9` _returnvalue :`10` _returnvalue)))

(fn `SetRoundManager`
  (bind _outactors (`GameplayStatics.GetAllActorsOfClass` "/Game/Blueprints/RoundManager.RoundManager_C"))
  (set `self.RoundManager` (`|GetArrayItem` _outactors)))

(fn `UserConstructionScript`)