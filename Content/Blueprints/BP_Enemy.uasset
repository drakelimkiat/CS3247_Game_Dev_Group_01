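; Enemy character whose goal state is full satisfaction rather than death: at 100 it reports to the RoundManager and destroys itself.
; ChangeSatisfaction adds progress and raises a short-lived hit flag, which Tick clears through a countdown.
; Tick also pushes the satisfaction value into its widget progress bar every frame.
; It finds the RoundManager on BeginPlay and provides a walk-speed setter that a Stop flag forces to zero.
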(event `self.ReceiveBeginPlay`
  (`self.SetRoundManager`))

(event `self.ReceiveTick`
  (params (DeltaSeconds :type "Float (single-precision)"))
  (bind _satisfaction (`self.Satisfaction`))
  (`self.ResetIsHit` DeltaSeconds)
  (bind _assatisfaction_bar (cast `/Game/SatisfactionBar` (`WidgetComponent.GetUserWidgetObject` (`self.SatisfactionBar`))))
  (`ProgressBar.SetPercent` (`/Game/SatisfactionBar.ProgressBar_18` _assatisfaction_bar) (/ _satisfaction 100.0))
  (if (>= _satisfaction 100.0)
    (`/Game/Blueprints/RoundManager.AddSatisfactions` (`self.RoundManager`))
    (`self.K2_DestroyActor`)))

(fn `ChangeSatisfaction`
  (params (Progress :type "Float (double-precision)"))
  (returns (something :type "Float (double-precision)"))
  (bind _output_get (set `self.Satisfaction` (+ Progress (`self.Satisfaction`))))
  (set `self.IsHIt` true)
  (set `self.IsHitResetTime` 0.05)
  (return _output_get))

(fn `ResetIsHit`
  (params (DeltaSeconds :type "Float (double-precision)"))
  (bind _ishitresettime (`self.IsHitResetTime`))
  (if (> _ishitresettime 0.0)
    (bind _output_get (set `self.IsHitResetTime` (- _ishitresettime DeltaSeconds)))
    (if (<= _output_get 0.0)
      (set `self.IsHIt` false))))

(fn `SetMaxWalkSpeed`
  (params (MaxWalkSpeed :type "Float (double-precision)"))
  (bind _charactermovement (`self.CharacterMovement`))
  (if (`self.Stop`)
    (set `CharacterMovementComponent.MaxWalkSpeed` 0.0 _charactermovement)
    (else
      (set `CharacterMovementComponent.MaxWalkSpeed` MaxWalkSpeed _charactermovement))))

(fn `SetRoundManager`
  (bind _outactors (`GameplayStatics.GetAllActorsOfClass` "/Game/Blueprints/RoundManager.RoundManager_C"))
  (set `self.RoundManager` (`|GetArrayItem` _outactors)))

(fn `UserConstructionScript`)