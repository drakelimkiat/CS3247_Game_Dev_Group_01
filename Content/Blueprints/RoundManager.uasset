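; Round manager actor that runs one of three enemy-spawning rounds and decides whether the level is won or lost.
; Each round spawns its mix of enemy types on timed delay loops at randomized radius-scaled positions; round one counts down, while two and three count up indefinitely.
; Complaint and satisfaction events update counters and the player's complaint bar.
; Tick checks those counters, triggering the HUD result and destroying the manager, plus all enemies on loss.
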(event `self.ReceiveBeginPlay`
  (bind _outactors (`GameplayStatics.GetAllActorsOfClass` "/Game/BP_HUD.BP_HUD_C"))
  (set `self.HUD` (`|GetArrayItem` _outactors))
  (`KismetSystemLibrary.Delay` 2.5)
  (bind _asfirst_person_character_1 (cast `/Game/FirstPersonBP/Blueprints/FirstPersonCharacter1` (`GameplayStatics.GetPlayerCharacter` 0)))
  (bind _output_get (set `self.PlayerCharacter` _asfirst_person_character_1))
  (`/Game/FirstPersonBP/Blueprints/FirstPersonCharacter1.Set ComplaintBar` _output_get 0.0)
  ;[1 1 1] Temporary Measure
  (`KismetSystemLibrary.PrintString` (`KismetStringLibrary.Concat_StrStr` "Round " (`KismetStringLibrary.Conv_IntToString` (`self.WhichRound`))))
  (set `self.Loop` (`self.TotalEnemy`))
  (switch `int` (`self.WhichRound`)
    (:`1`
      (`self.RoundOne`))
    (:`2`
      (`self.RoundTwo`))
    (:`3`
      (`self.RoundThree`))))

(event `self.ReceiveTick`
  (params (DeltaSeconds :type "Float (single-precision)"))
  (if (>= (`self.NumOfComplaints`) (`self.MaxComplaints`))
    (`self.GameOver`)
    (elif (== (+ (`self.NumOfComplaints`) (`self.NumOfSatisfactions`)) (`self.TotalEnemy`))
      (`self.GameClear`))))

(event `AddComplaints`
  (bind _result (`/Engine/EditorBlueprintResources/StandardMacros.IncrementInt` (`self.NumOfComplaints`))
    (:`  `
      (`/Game/FirstPersonBP/Blueprints/FirstPersonCharacter1.Set ComplaintBar` (`self.PlayerCharacter`) (/ (`KismetMathLibrary.Conv_IntToDouble` _result) (`KismetMathLibrary.Conv_IntToDouble` (`self.MaxComplaints`))))
      ;[1 1 1] Temporary Measure
      (`KismetSystemLibrary.PrintString` (`KismetStringLibrary.Concat_StrStr` "Complaints: " (`KismetStringLibrary.Conv_IntToString` _result))))))

(event `AddSatisfactions`
  (bind _result (`/Engine/EditorBlueprintResources/StandardMacros.IncrementInt` (`self.NumOfSatisfactions`))
    (:`  `
      ;[1 1 1] Temporary Measure
      (`KismetSystemLibrary.PrintString` (`KismetStringLibrary.Concat_StrStr` "Satisfactions:" (`KismetStringLibrary.Conv_IntToString` _result))))))

(event `RoundOne`
  (bind _loop (`self.Loop`))
  (`KismetSystemLibrary.Delay` 5.0)
  (`self.HideHUD`)
  (if (> _loop 0) :!label _label
    (`KismetSystemLibrary.Delay` 10.0)
    (`self.SpawnEnemyAverageJoe`)
    (`/Engine/EditorBlueprintResources/StandardMacros.DecrementInt` _loop
      (:`  `
        (goto _label)))))

(event `RoundTwo`
  (bind _loop (`self.Loop`))
  (`KismetSystemLibrary.Delay` 5.0)
  (`self.HideHUD`)
  (if (> _loop 0) :!label _label_2
    (switch `int` (mod _loop 2)
      (:`0`
        (`KismetSystemLibrary.Delay` 10.0)
        (`self.SpawnEnemyKid`))
      (:`1`
        (`KismetSystemLibrary.Delay` 8.0)
        (`self.SpawnEnemyAverageJoe`)))
    (`/Engine/EditorBlueprintResources/StandardMacros.IncrementInt` _loop
      (:`  `
        (goto _label_2)))))

(event `RoundThree`
  (bind _loop (`self.Loop`))
  (`KismetSystemLibrary.Delay` 5.0)
  (`self.HideHUD`)
  (if (> _loop 0) :!label _label_3
    (switch `int` (mod _loop 4)
      (:`0`
        (`KismetSystemLibrary.Delay` 10.0)
        (`self.SpawnEnemyAverageJoe`))
      (:`1`
        (`KismetSystemLibrary.Delay` 8.0)
        (`self.SpawnEnemyGymDude`))
      (:`2`
        (`KismetSystemLibrary.Delay` 8.0)
        (`self.SpawnEnemyAverageJoe`))
      (:`3`
        (`KismetSystemLibrary.Delay` 10.0)
        (`self.SpawnEnemyKid`)))
    (`/Engine/EditorBlueprintResources/StandardMacros.IncrementInt` _loop
      (:`  `
        (goto _label_3)))))

(event `GameClear`
  (bind _hud (`self.HUD`))
  ;[1 1 1] Temporary Measure
  (`KismetSystemLibrary.PrintString` "You won the level!")
  (set `/Game/BP_HUD.Display?` true _hud)
  (set `/Game/BP_HUD.Cleared?` true _hud)
  (`self.K2_DestroyActor`))

(event `GameOver`
  (bind _hud (`self.HUD`))
  ;[1 1 1] Temporary Measure
  (`KismetSystemLibrary.PrintString` "You lost the level:/")
  (set `/Game/BP_HUD.Display?` true _hud)
  (set `/Game/BP_HUD.Cleared?` false _hud)
  (bind _outactors (`GameplayStatics.GetAllActorsOfClass` "/Game/Blueprints/BP_Enemy.BP_Enemy_C"))
  (for _array_element _outactors
    (`self.K2_DestroyActor` _array_element))
  (`self.K2_DestroyActor`))

(fn `GetSpawnTransform`
  (params (EnemyHalfHeight :type "Float (double-precision)"))
  (returns (SpawnTransform :type "Transform Structure"))
  (bind _returnvalue (`KismetMathLibrary.RandomFloatInRange` 0.0 180.0))
  (bind _spawnenemyradius (`self.SpawnEnemyRadius`))
  (return (`KismetMathLibrary.MakeTransform` (`KismetMathLibrary.MakeVector` (* (`KismetMathLibrary.DegSin` _returnvalue) _spawnenemyradius) (* (`KismetMathLibrary.DegCos` _returnvalue) _spawnenemyradius) EnemyHalfHeight) (`KismetMathLibrary.MakeRotator` 0.0 0.0 (- -90.0 _returnvalue)))))

(fn `HideHUD`
  (set `/Game/BP_HUD.Display?` false (`self.HUD`)))

(fn `SpawnEnemyAverageJoe`
  (bind _spawntransform (`self.GetSpawnTransform` (`self.EnemyAverageJoeHalfHeight`)))
  (`|SpawnActorFromClass` "/Game/Blueprints/BP_EnemyAverageJoe.BP_EnemyAverageJoe_C" _spawntransform "AdjustIfPossibleButDontSpawnIfColliding" "OverrideRootScale" null null))

(fn `SpawnEnemyGymDude`
  (bind _spawntransform (`self.GetSpawnTransform` (`self.EnemyGymDudeHalfHeight`)))
  (`|SpawnActorFromClass` "/Game/Blueprints/BP_EnemyGymDude.BP_EnemyGymDude_C" _spawntransform "AdjustIfPossibleButDontSpawnIfColliding" "OverrideRootScale" null null))

(fn `SpawnEnemyKid`
  (bind _spawntransform (`self.GetSpawnTransform` (`self.EnemyKidHalfHeight`)))
  (`|SpawnActorFromClass` "/Game/Blueprints/BP_EnemyKid.BP_EnemyKid_C" _spawntransform "AdjustIfPossibleButDontSpawnIfColliding" "OverrideRootScale" null null))

(fn `UserConstructionScript`)