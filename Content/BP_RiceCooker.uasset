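; Rice cooker station that takes undone BP_Food_RiceCooker items from the player's hand, cooks them and hands them back.
; Interact snaps food in, returns it or swaps it while the lid is open.
; Tick uses a DoOnce to close the lid and start a looping timer filling the level's BP_RiceCookerBar, then at full marks food done, opens the lid and rings a bell.
; Also toggles a custom-depth placement outline and tutorial arrow.
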(event `OpenLid`
  ;[1 1 1] Open lid
  (bind (_direction _open) (`Timeline|OpenRotation` :!via `PlayFromStart`)
    (:`Update`
      (`SceneComponent.K2_SetRelativeRotation` (`self.Lid`) (`KismetMathLibrary.MakeRotator` 0.0 _open) false false)
      (set `self.LidOpen` true))))

(event `CloseLid`
  ;[1 1 1] Close lid
  (bind (_direction _close) (`Timeline|CloseRotation` :!via `PlayFromStart`)
    (:`Update`
      (`SceneComponent.K2_SetRelativeRotation` (`self.Lid`) (`KismetMathLibrary.MakeRotator` 0.0 _close) false false)
      (set `self.LidOpen` false))))

(event `self.ReceiveBeginPlay`
  ;[1 1 1] On begin play: set RiceCookerBar
  (bind _outactors (`GameplayStatics.GetAllActorsOfClass` "/Game/BP_RiceCookerBar.BP_RiceCookerBar_C"))
  (set `self.RiceCookerBar` (`|GetArrayItem` _outactors)))

(event `self.ReceiveTick`
  (params (DeltaSeconds :type "Float (single-precision)"))
  (bind _widget (`/Game/BP_RiceCookerBar.Widget` (`self.RiceCookerBar`)))
  ;[1 1 1] If food i placed in rice cooker: start timer and make rice visible.
  (if (`self.HasFoodInIt?`)
    (`SceneComponent.SetVisibility` _widget true false)
    (`SceneComponent.SetVisibility` (`self.Rice`) true false)
    (if (>= (`/Game/BP_RiceCookerBar.Progress` (`self.RiceCookerBar`)) 100.0)
      (bind _asbp_food (cast `/Game/FoodBP/BP_Food` (`self.Food`)))
      (if (not (`/Game/FoodBP/BP_Food.Done` _asbp_food))
        (set `/Game/FoodBP/BP_Food.Done` true _asbp_food)
        (`self.OpenLid`)
        (`GameplayStatics.PlaySoundAtLocation` "/Game/Sound/bell_Cue.bell_Cue" (`SceneComponent.K2_GetComponentLocation` (`self.Body`)) (struct) 0.5)
        (`KismetSystemLibrary.K2_ClearAndInvalidateTimerHandle` (stale _returnvalue))
        (goto _label :!via `Reset`))
      (else
        (`/Engine/EditorBlueprintResources/StandardMacros.DoOnce` false :!label _label
          (:`Completed`
            (`self.CloseLid`)
            (bind _asbp_food_rice_cooker (cast `/Game/FoodBP/BP_Food_RiceCooker` (`self.Food`)))
            (bind _returnvalue (`KismetSystemLibrary.K2_SetTimer` null "Cook" (/ (`/Game/FoodBP/BP_Food_RiceCooker.PreparationTime` _asbp_food_rice_cooker) 20.0) true))))))
    (else
      (`SceneComponent.SetVisibility` _widget false false)
      (`SceneComponent.SetVisibility` (`self.Rice`) false false)
      (`/Game/BP_RiceCookerBar.ResetRiceCookerBar` (`self.RiceCookerBar`)))))

(event `/Game/BPI_OutlineOnFood.SetOutlineOn`
  (params (Food :type "Actor Object Reference"))
  ;[1 1 1] Give rice cooker green outline if food in hand can be placed on board.
  (if (`KismetMathLibrary.ClassIsChildOf` (`GameplayStatics.GetObjectClass` Food) "/Game/FoodBP/BP_Food_RiceCooker.BP_Food_RiceCooker_C")
    (if (not (`self.HasFoodInIt?`))
      (bind _asbp_food_rice_cooker (cast `/Game/FoodBP/BP_Food_RiceCooker` Food))
      (if (not (`/Game/FoodBP/BP_Food.Done` _asbp_food_rice_cooker))
        (`PrimitiveComponent.SetRenderCustomDepth` (`self.Body`) true)
        (set `self.OutlineOn` true)))))

(event `/Game/BPI_OutlineOff.SetOutlineOff`
  ;[1 1 1] Remove green outline when hand is not touching cooker.
  (if (`self.OutlineOn`)
    (`PrimitiveComponent.SetRenderCustomDepth` (`self.Body`) false)
    (set `self.OutlineOn` false)))

(event `/Game/BPI_InteractLeft.Interact`
  (bind _food (`self.Food`))
  ;[1 1 1] When player interacts with frying pan
  (if (`self.HasFoodInIt?`)
    (if (`self.LidOpen`)
      (bind _asfirst_person_character_1 (cast `/Game/FirstPersonBP/Blueprints/FirstPersonCharacter1` (`GameplayStatics.GetPlayerCharacter` 0)))
      (`/Engine/EditorBlueprintResources/StandardMacros.IsValid` _food
        (:`Is Valid`
          (bind _food_2 (`/Game/FirstPersonBP/Blueprints/FirstPersonCharacter1.Food` _asfirst_person_character_1))
          (`/Engine/EditorBlueprintResources/StandardMacros.IsValid` _food_2
            (:`Is Valid`
              (bind _asbp_food (cast `/Game/FoodBP/BP_Food` _food_2))
              (if (`/Game/FoodBP/BP_Food.Done` _asbp_food)
                _
                (elif (`KismetMathLibrary.ClassIsChildOf` (`GameplayStatics.GetObjectClass` _asbp_food) "/Game/FoodBP/BP_Food_RiceCooker.BP_Food_RiceCooker_C")
                  (`self.K2_SetActorTransform` _asbp_food (`KismetMathLibrary.MakeTransform` (.location (`SceneComponent.K2_GetComponentToWorld` (`self.SnapPoint`))) (.rotation (`SceneComponent.K2_GetComponentToWorld` (`self.SnapPoint`)))) false false)
                  (set `/Game/FirstPersonBP/Blueprints/FirstPersonCharacter1.Food` _food _asfirst_person_character_1)
                  (set `/Game/FirstPersonBP/Blueprints/FirstPersonCharacter1.HoldingFood` true _asfirst_person_character_1)
                  (set `self.Food` _asbp_food)
                  (set `self.HasFoodInIt?` true)
                  (`/Game/BP_RiceCookerBar.ResetRiceCookerBar` (`self.RiceCookerBar`))
                  (goto _label :!via `Reset`))))
            (:`Is Not Valid`
              (set `/Game/FirstPersonBP/Blueprints/FirstPersonCharacter1.Food` _food _asfirst_person_character_1)
              (set `/Game/FirstPersonBP/Blueprints/FirstPersonCharacter1.HoldingFood` true _asfirst_person_character_1)
              (set `self.Food` null)
              (set `self.HasFoodInIt?` false))))))
    (else
      (`self.DropFood`))))

(event `/Game/BPI_TutorialIndicatorOn.SetTutorialIndicatorOn`
  ;[1 1 1] Tutorial: Arrow on/off
  (`/Engine/EditorBlueprintResources/StandardMacros.IsValid` (`self.Arrow`)
    (:`Is Not Valid`
      (bind _returnvalue (`|SpawnActorFromClass` "/Game/BP_Tutorial_Arrow.BP_Tutorial_Arrow_C" (`KismetMathLibrary.MakeTransform` (+ (`SceneComponent.K2_GetComponentLocation` (`self.SnapPoint`)) (0.0 5.0 0.0))) "Undefined" "OverrideRootScale" null null))
      (set `self.Arrow` _returnvalue))))

(event `/Game/BPI_TutorialIndicatorOff.SetTutorialIndicatorOff`
  ;[1 1 1] Tutorial: Arrow on/off
  (`self.K2_DestroyActor` (`self.Arrow`)))

(fn `Cook`
  (`/Game/BP_RiceCookerBar.IncreaseRiceCookerBar` (`self.RiceCookerBar`) 5.0))

(fn `DropFood`
  (bind _asfirst_person_character_1 (cast `/Game/FirstPersonBP/Blueprints/FirstPersonCharacter1` (`GameplayStatics.GetPlayerCharacter` 0)))
  (bind _asbp_food (cast `/Game/FoodBP/BP_Food` (`/Game/FirstPersonBP/Blueprints/FirstPersonCharacter1.Food` _asfirst_person_character_1)))
  (if (`/Game/FoodBP/BP_Food.Done` _asbp_food)
    _
    (elif (`KismetMathLibrary.ClassIsChildOf` (`GameplayStatics.GetObjectClass` _asbp_food) "/Game/FoodBP/BP_Food_RiceCooker.BP_Food_RiceCooker_C")
      (`self.K2_SetActorTransform` _asbp_food (`KismetMathLibrary.MakeTransform` (.location (`SceneComponent.K2_GetComponentToWorld` (`self.SnapPoint`))) (.rotation (`SceneComponent.K2_GetComponentToWorld` (`self.SnapPoint`)))) false false)
      (set `/Game/FirstPersonBP/Blueprints/FirstPersonCharacter1.Food` null _asfirst_person_character_1)
      (set `/Game/FirstPersonBP/Blueprints/FirstPersonCharacter1.HoldingFood` false _asfirst_person_character_1)
      (set `self.Food` _asbp_food)
      (set `self.HasFoodInIt?` true))))

(fn `UserConstructionScript`)