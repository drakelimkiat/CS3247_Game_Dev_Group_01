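; Trash bin where the player discards held food, with a lid that reacts to the player's hand.
; Box overlaps with the character's Hand or VRHand trigger the Open and Close timelines, which pitch the Lid and set LidOpen.
; Interact clears the character's held food state and destroys the BP_Food actor.
; Tutorial events spawn or destroy a single BP_TutorialArrow at SnapPoint.
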(event `OpenLid`
  ;[1 1 1] Open lid
  (bind (_direction _open) (`Timeline|Open` :!via `PlayFromStart`)
    (:`Update`
      (`SceneComponent.K2_SetRelativeRotation` (`self.Lid`) (`KismetMathLibrary.MakeRotator` 0.0 _open) false false)
      (set `self.LidOpen` true))))

(event `/Game/BPI_TutorialIndicatorOn.SetTutorialIndicatorOn`
  ;[1 1 1] Tutorial: Arrow on/off
  (`/Engine/EditorBlueprintResources/StandardMacros.IsValid` (`self.Arrow`)
    (:`Is Not Valid`
      (bind _returnvalue (`|SpawnActorFromClass` "/Game/BP_TutorialArrow.BP_TutorialArrow_C" (`KismetMathLibrary.MakeTransform` (`SceneComponent.K2_GetComponentLocation` (`self.SnapPoint`)) (struct :`Yaw` 90.0)) "Undefined" "OverrideRootScale" null null))
      (set `self.Arrow` _returnvalue))))

(event `CloseLid`
  ;[1 1 1] Close lid
  (bind (_direction _close) (`Timeline|Close` :!via `PlayFromStart`)
    (:`Update`
      (`SceneComponent.K2_SetRelativeRotation` (`self.Lid`) (`KismetMathLibrary.MakeRotator` 0.0 _close) false false)
      (set `self.LidOpen` false))))

(event `/Game/BPI_TutorialIndicatorOff.SetTutorialIndicatorOff`
  (bind _arrow (`self.Arrow`))
  ;[1 1 1] Tutorial: Arrow on/off
  (`/Engine/EditorBlueprintResources/StandardMacros.IsValid` _arrow
    (:`Is Valid`
      (`self.K2_DestroyActor` _arrow))))

(event `/Game/BPI_InteractLeft.Interact`
  ;[1 1 1] Throw food in trash
  (bind _asfirst_person_character_1 (cast `/Game/FirstPersonBP/Blueprints/FirstPersonCharacter1` (`GameplayStatics.GetPlayerCharacter` 0)))
  (bind _asbp_food (cast `/Game/FoodBP/BP_Food` (`/Game/FirstPersonBP/Blueprints/FirstPersonCharacter1.Food` _asfirst_person_character_1)))
  (set `/Game/FirstPersonBP/Blueprints/FirstPersonCharacter1.Food` null _asfirst_person_character_1)
  (set `/Game/FirstPersonBP/Blueprints/FirstPersonCharacter1.HoldingFood` false _asfirst_person_character_1)
  (`self.K2_DestroyActor` _asbp_food))

(event `self.Box.OnComponentBeginOverlap`
  (params (OverlappedComponent :type "PrimitiveComponent Object Reference") (OtherActor :type "Actor Object Reference") (OtherComp :type "PrimitiveComponent Object Reference") (OtherBodyIndex :type Integer) (bFromSweep :type Boolean) (SweepResult :type "HitResult Structure (by ref)"))
  ;[1 1 1] Open/close lid when hand is overlaping
  (bind _asfirst_person_character_1 (cast `/Game/FirstPersonBP/Blueprints/FirstPersonCharacter1` (`GameplayStatics.GetPlayerCharacter` 0)))
  (if (== (`/Game/FirstPersonBP/Blueprints/FirstPersonCharacter1.Hand` _asfirst_person_character_1) OtherComp)
    (`self.OpenLid` :!label _label)
    (elif (== (`/Game/FirstPersonBP/Blueprints/FirstPersonCharacter1.VR_Hand` _asfirst_person_character_1) OtherComp)
      (goto _label))))

(event `self.Box.OnComponentEndOverlap`
  (params (OverlappedComponent :type "PrimitiveComponent Object Reference") (OtherActor :type "Actor Object Reference") (OtherComp :type "PrimitiveComponent Object Reference") (OtherBodyIndex :type Integer))
  ;[1 1 1] Open/close lid when hand is overlaping
  (bind _asfirst_person_character_1 (cast `/Game/FirstPersonBP/Blueprints/FirstPersonCharacter1` (`GameplayStatics.GetPlayerCharacter` 0)))
  (if (== (`/Game/FirstPersonBP/Blueprints/FirstPersonCharacter1.Hand` _asfirst_person_character_1) OtherComp)
    (`self.CloseLid` :!label _label_2)
    (elif (== (`/Game/FirstPersonBP/Blueprints/FirstPersonCharacter1.VR_Hand` _asfirst_person_character_1) OtherComp)
      (goto _label_2))))

(fn `UserConstructionScript`)