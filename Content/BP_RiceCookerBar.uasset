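; BP_RiceCookerBar is an actor that displays rice cooker progress through a FoodRiceCookerBar widget hosted on its Widget component.
; Every Tick casts the component's user widget and sets its progress bar to Progress divided by 100.
; IncreaseRiceCookerBar is the function for adding to Progress, and ResetRiceCookerBar sets it back to zero.
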(event `self.ReceiveTick`
  (params (DeltaSeconds :type "Float (single-precision)"))
  (bind _asfood_rice_cooker_bar (cast `/Game/FoodRiceCookerBar` (`WidgetComponent.GetUserWidgetObject` (`self.Widget`))))
  (`ProgressBar.SetPercent` (`/Game/FoodRiceCookerBar.ProgressBar_18` _asfood_rice_cooker_bar) (/ (`self.Progress`) 100.0)))

(fn `IncreaseRiceCookerBar`
  (params (Progress :type "Float (double-precision)"))
  (set `self.Progress` (+ Progress (`self.Progress`))))

(fn `ResetRiceCookerBar`
  (set `self.Progress` 0.0))

(fn `UserConstructionScript`)