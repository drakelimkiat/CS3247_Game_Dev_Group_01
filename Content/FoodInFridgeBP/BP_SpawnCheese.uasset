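; BP_SpawnCheese is a food spawner child Blueprint in the fridge food set that supplies cheese.
; On BeginPlay it runs the parent logic, then sets the spawn class to BP_Food_Cheese and the spawn transform to the Cheese component's world transform.
; It contains no spawn call of its own, and its overlap and tick events are disabled.
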(event `self.ReceiveBeginPlay`
  ;[1 1 1] Set what food to be spawned and where.
  (`parent.ReceiveBeginPlay`)
  (set `self.SpawnClass` "/Game/FoodBP/BP_Food_Cheese.BP_Food_Cheese_C")
  (set `self.SpawnTransform` (`SceneComponent.K2_GetComponentToWorld` (`self.Cheese`))))

(fn `UserConstructionScript`
  (`parent.UserConstructionScript`))