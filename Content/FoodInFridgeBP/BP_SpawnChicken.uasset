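; BP_SpawnChicken is a food spawner Blueprint for chicken, part of the food-in-fridge set.
; On BeginPlay it runs the parent logic, then sets SpawnClass to BP_Food_Chicken and SpawnTransform to the world transform of its Ch1 component.
; It only configures what and where to spawn; no spawn call appears in this Blueprint, and its overlap and Tick events are disabled.
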(event `self.ReceiveBeginPlay`
  ;[1 1 1] Set which food to spawn and where.
  (`parent.ReceiveBeginPlay`)
  (set `self.SpawnClass` "/Game/FoodBP/BP_Food_Chicken.BP_Food_Chicken_C")
  (set `self.SpawnTransform` (`SceneComponent.K2_GetComponentToWorld` (`self.Ch1`))))

(fn `UserConstructionScript`
  (`parent.UserConstructionScript`))