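; BP_Spawn is an interactable actor that spawns food for the player while the fridge door is open.
; On BeginPlay it caches the first BP_Fridge found in the level.
; Interact checks that fridge's DoorOpen flag, prints a debug string and spawns SpawnClass at SpawnTransform.
; The new actor is stored as Food on FirstPersonCharacter1, which is flagged as holding food.
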(event `self.ReceiveBeginPlay`
  (bind _outactors (`GameplayStatics.GetAllActorsOfClass` "/Game/BP_Fridge.BP_Fridge_C"))
  (set `self.Fridge` (`|GetArrayItem` _outactors)))

(event `/Game/BPI_InteractLeft.Interact`
  (if (`/Game/BP_Fridge.DoorOpen` (`self.Fridge`))
    (`KismetSystemLibrary.PrintString` "Hello" true true (struct :`R` 1.0 :`G` 0.227199 :`B` 0.799711 :`A` 1.0))
    (bind _returnvalue (`|SpawnActorFromClass` (`self.SpawnClass`) (`self.SpawnTransform`) "Undefined" "OverrideRootScale" null null))
    (bind _asfirst_person_character_1 (cast `/Game/FirstPersonBP/Blueprints/FirstPersonCharacter1` (`GameplayStatics.GetPlayerCharacter` 0)))
    (set `/Game/FirstPersonBP/Blueprints/FirstPersonCharacter1.Food` _returnvalue _asfirst_person_character_1)
    (set `/Game/FirstPersonBP/Blueprints/FirstPersonCharacter1.HoldingFood` true _asfirst_person_character_1)))

(fn `UserConstructionScript`)