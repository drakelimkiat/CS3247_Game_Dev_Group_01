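; BP_FryingBar is a progress bar display for food frying, built on a widget component that hosts a FoodFryingBar widget.
; Every Tick it casts the widget and sets its progress bar from the Progress variable, treated as a 0–100 percentage.
; IncreaseFryingBar and ResetFryingBar are the functions that raise and zero Progress, with no clamping or frying logic in this Blueprint.
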(event `self.ReceiveTick`
  (params (DeltaSeconds :type "Float (single-precision)"))
  (bind _asfood_frying_bar (cast `/Game/FoodFryingBar` (`WidgetComponent.GetUserWidgetObject` (`self.Widget`))))
  (`ProgressBar.SetPercent` (`/Game/FoodFryingBar.ProgressBar_18` _asfood_frying_bar) (/ (`self.Progress`) 100.0)))

(fn `increaseFryingBar`
  (params (Progress :type "Float (double-precision)"))
  (set `self.Progress` (+ Progress (`self.Progress`))))

(fn `ResetFryingBar`
  (set `self.Progress` 0.0))

(fn `UserConstructionScript`)