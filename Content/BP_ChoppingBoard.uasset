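; BP_ChoppingBoard is an interactable cooking station that holds a food item for chopping.
; Interacting hands the board's food to the first-person player character and clears the board.
; Chop advances a BP_ChoppingBar progress meter, found in the level at BeginPlay.
; Tick shows that bar's widget while food is on the board, otherwise hiding and resetting it every frame.
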(event `/Game/BPI_InteractLeft.Interact`
  (bind _asfirst_person_character_1 (cast `/Game/FirstPersonBP/Blueprints/FirstPersonCharacter1` (`GameplayStatics.GetPlayerCharacter` 0)))
  (set `/Game/FirstPersonBP/Blueprints/FirstPersonCharacter1.Food` (`self.Food`) _asfirst_person_character_1)
  (set `/Game/FirstPersonBP/Blueprints/FirstPersonCharacter1.HoldingFood` true _asfirst_person_character_1)
  (set `self.Food` null)
  (set `self.HasFoodOnTop?` false))

(event `self.ReceiveBeginPlay`
  (bind _outactors (`GameplayStatics.GetAllActorsOfClass` "/Game/BP_ChoppingBar.BP_ChoppingBar_C"))
  (set `self.ChoppingBar` (`|GetArrayItem` _outactors)))

(event `self.ReceiveTick`
  (params (DeltaSeconds :type "Float (single-precision)"))
  (bind _widget (`/Game/BP_ChoppingBar.Widget` (`self.ChoppingBar`)))
  (if (`self.HasFoodOnTop?`)
    (`SceneComponent.SetVisibility` _widget true false)
    (else
      (`SceneComponent.SetVisibility` _widget false false)
      (`/Game/BP_ChoppingBar.ResetChoppingBar` (`self.ChoppingBar`)))))

(fn `Chop`
  (`/Game/BP_ChoppingBar.IncreaseChoppingBar` (`self.ChoppingBar`) 10.0))

(fn `UserConstructionScript`)