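; BP_Instructions is a world-placed instruction display with a mesh and a widget component that keep facing the player character.
; Every tick it computes a look-at yaw toward the player for each component and applies only that yaw, with the mesh offset by 90 degrees.
; SetInstructionText casts the widget to InstructionsWidget and writes the passed text into its multi-line text box.
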(event `self.ReceiveTick`
  (params (DeltaSeconds :type "Float (single-precision)"))
  (bind (_returnvalue_roll _returnvalue_pitch _returnvalue_yaw) (`KismetMathLibrary.BreakRotator` (`KismetMathLibrary.FindLookAtRotation` (`SceneComponent.K2_GetComponentLocation` (`self.Mesh`)) (`self.K2_GetActorLocation` (`GameplayStatics.GetPlayerCharacter` 0)))))
  (bind (_returnvalue_roll_2 _returnvalue_pitch_2 _returnvalue_yaw_2) (`KismetMathLibrary.BreakRotator` (`KismetMathLibrary.FindLookAtRotation` (`SceneComponent.K2_GetComponentLocation` (`self.Widget`)) (`self.K2_GetActorLocation` (`GameplayStatics.GetPlayerCharacter` 0)))))
  (`SceneComponent.K2_SetWorldRotation` (`self.Widget`) (`KismetMathLibrary.MakeRotator` 0.0 0.0 _returnvalue_yaw_2) false false)
  (`SceneComponent.K2_SetWorldRotation` (`self.Mesh`) (`KismetMathLibrary.MakeRotator` 0.0 0.0 (- _returnvalue_yaw 90.0)) false false))

(fn `SetInstructionText`
  (params (Text :type Text))
  (bind _asinstructions_widget (cast `/Game/InstructionsWidget` (`WidgetComponent.GetUserWidgetObject` (`self.Widget`))))
  (`MultiLineEditableText.SetText` (`/Game/InstructionsWidget.MultiLineEditableText_35` _asinstructions_widget) Text))

(fn `UserConstructionScript`)