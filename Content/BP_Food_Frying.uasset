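; Food actor that cooks after touching a BP_Pan and swaps to its finished mesh when done.
; A pan hit shows the progress bar and starts a looping one-second timer that counts down TimeLeft.
; Tick yaws the bar toward the player, fills it from TimeLeft over PreparationTime, then pauses the timer and sets Done at zero.
; Nothing pauses cooking when the food leaves the pan.
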(event `self.ReceiveBeginPlay`)

(event `self.ReceiveTick`
  (params (DeltaSeconds :type "Float (single-precision)"))
  (bind _progressbar (`self.ProgressBar`))
  ;[1 1 1] Make progress bar face player
  (`SceneComponent.K2_SetWorldRotation` _progressbar (`KismetMathLibrary.MakeRotator` 0.0 0.0 (.yaw (`KismetMathLibrary.FindLookAtRotation` (`SceneComponent.K2_GetComponentLocation` _progressbar) (`self.K2_GetActorLocation` (`GameplayStatics.GetPlayerPawn` 0))))) false false)
  (if (not (`self.Done`))
    ;[1 1 1] If food is not done: Fill progress bar
    (bind _asfood_frying_bar (cast `/Game/FoodFryingBar` (`WidgetComponent.GetUserWidgetObject` (`self.ProgressBar`))))
    (`ProgressBar.SetPercent` (`/Game/FoodFryingBar.ProgressBar_18` _asfood_frying_bar) (- 1.0 (/ (`self.TimeLeft`) (`self.PreparationTime`))))
    ;[1 1 1] Check if the food is supposed to be done
    (if (<= (`self.TimeLeft`) 0.0)
      ;[1 1 1] If food is done: Change static mesh to MeshDone
      (`StaticMeshComponent.SetStaticMesh` (`self.Food`) (`self.MeshDone`))
      (`KismetSystemLibrary.K2_PauseTimer` null "Frying")
      (set `self.Done` true))))

(event `self.Food.OnComponentHit`
  (params (HitComponent :type "PrimitiveComponent Object Reference") (OtherActor :type "Actor Object Reference") (OtherComp :type "PrimitiveComponent Object Reference") (NormalImpulse :type "Vector Structure") (Hit :type "HitResult Structure (by ref)"))
  ;[1 1 1] If food hit pan: Start timer and make progress bar vissible
  (if (== (`GameplayStatics.GetObjectClass` OtherActor) "/Game/BP_Pan.BP_Pan_C")
    (`KismetSystemLibrary.K2_SetTimer` null "Frying" 1.0 true)
    (`SceneComponent.SetVisibility` (`self.ProgressBar`) true false)))

(fn `Frying`
  (set `self.TimeLeft` (- (`self.TimeLeft`) 1.0)))

(fn `UserConstructionScript`)