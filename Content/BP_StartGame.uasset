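; BP_StartGame is an interactable start-game object that launches the ChopItLikeItsHot level.
; Interact starts a fade on the player camera and opens the level by name right away.
; SetOutlineon and SetOutlineOff toggle custom depth on its Game and Start components to show or hide a green outline highlight.
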(event `/Game/BPI_InteractLeft.Interact`
  (`PlayerCameraManager.StartCameraFade` :`self` (`GameplayStatics.GetPlayerCameraManager` 0))
  (`GameplayStatics.OpenLevel` "ChopItLikeItsHot"))

(event `/Game/BPI_OutlineOnNoFood.SetOutlineOn`
  ;[1 1 1] Green outline on and off.
  (`PrimitiveComponent.SetRenderCustomDepth` (`self.Game`) true)
  (`PrimitiveComponent.SetRenderCustomDepth` (`self.Start`) true))

(event `/Game/BPI_OutlineOff.SetOutlineOff`
  ;[1 1 1] Green outline on and off.
  (`PrimitiveComponent.SetRenderCustomDepth` (`self.Game`) false)
  (`PrimitiveComponent.SetRenderCustomDepth` (`self.Start`) false))

(fn `UserConstructionScript`)